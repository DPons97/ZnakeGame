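; Player snake character that moves in 32-unit steps and reports game over to BP_ZnakeGameMode on hitting body or Layer_2 map pieces.
; Tick applies acceleration to Speed and fires steps at 1/Speed intervals, once a direction input opens the gate.
; Each unblocked step passes the previous transform down the body chain created at BeginPlay.
; Inputs also pause the game and activate the first pooled ability, with a cooldown.
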(event EventBeginPlay
  ;[1 1 1] Initialization
  (for _index (range 0 2)
    (CallFunction|InitSnake _index)))

(event EventTick
  (params (DeltaSeconds :type Float%20%28single-precision%29))
  ;[1 1 1] Movement
  (Utilities|UpdateSpeedifAccelerating DeltaSeconds)
  (Utilities|IsSpeedTimerExpired DeltaSeconds
    (:True
      (Utilities|FlowControl|Gate true
        (:Exit
          (switch int (Variables|Default|GetMovementDirection)
            (:0
              (CallFunction|MoveForward 0.0))
            (:1
              (CallFunction|MoveForward 1.8e+02))
            (:2
              (CallFunction|MoveForward 9e+01))
            (:3
              (CallFunction|MoveForward -9e+01))))))))

(event Input|ActionEvents|InputActionUp
  (params (Key :type Key%20Structure))
  ;[1 1 1] Movement
  (:Pressed
    (Variables|Default|SetMovementDirection 0)
    (Utilities|FlowControl|Gate true) ; enters at Open
  ))

(event Input|ActionEvents|InputActionCastAbility
  (params (Key :type Key%20Structure))
  ;[1 1 1] Other Inputs
  (:Pressed
    (Utilities|CastAbility)))

(event Input|ActionEvents|InputActionPause
  (params (Key :type Key%20Structure))
  ;[1 1 1] Other Inputs
  (:Pressed
    (Default|PauseGame (Variables|Default|GetGameModeReference))))

(event Input|ActionEvents|InputActionRight
  (params (Key :type Key%20Structure))
  ;[1 1 1] Movement
  (:Pressed
    (Variables|Default|SetMovementDirection 2)
    (Utilities|FlowControl|Gate true) ; enters at Open
  ))

(event Input|ActionEvents|InputActionLeft
  (params (Key :type Key%20Structure))
  ;[1 1 1] Movement
  (:Pressed
    (Variables|Default|SetMovementDirection 3)
    (Utilities|FlowControl|Gate true) ; enters at Open
  ))

(event Input|ActionEvents|InputActionDown
  (params (Key :type Key%20Structure))
  ;[1 1 1] Movement
  (:Pressed
    (Variables|Default|SetMovementDirection 1)
    (Utilities|FlowControl|Gate true) ; enters at Open
  ))

(fn ConstructionScript)

(fn MoveForward
  (params (Direction :type Float%20%28single-precision%29))
  (bind _returnvalue (Transformation|GetActorRotation))
  (bind (_roll _pitch) (Math|Rotator|BreakRotator _returnvalue))
  (bind _correcteddirection (Utilities|IsMovingBackwards Direction)
    (:True
      _)
    (:False
      (Variables|Default|SetDirection _correcteddirection)))
  (Variables|Default|SetLastTransform (Transformation|GetActorTransform))
  (Pawn|SetControlRotation (Pawn|GetController) (Math|Rotator|MakeRotator _roll _pitch (Variables|Default|GetDirection)))
  (bind _sweephitresult (Transformation|AddActorLocalOffset "32.000000, 0, 0" true false))
  (if (.bBlockingHit (Collision|BreakHitResult _sweephitresult))
    (bind _output_get (Variables|Default|SetHitActor (.HitActor (Collision|BreakHitResult _sweephitresult))))
    (if (Actor|ActorHasTag _output_get "Body")
      (CallFunction|SnakeGameOver)
      (elif (Actor|ActorHasTag (Variables|Default|GetHitActor) "Map")
        (bind _output_get_2 (Variables|Default|SetHitComponent (.HitComponent (Collision|BreakHitResult _sweephitresult))))
        (if (Components|ComponentHasTag _output_get_2 "Layer_2")
          (CallFunction|SnakeGameOver))))
    (else
      (Default|MovetoNextTile (Variables|Default|GetNextBodyRef) (Variables|Default|GetLastTransform)))))

(fn InitSnake
  (params (Index :type Integer))
  (bind _returnvalue (Transformation|GetActorTransform))
  (bind _returnvalue_2 (Math|Vector|MakeVector 32.0 0.0 0.0))
  (bind _returnvalue_3 (Math|Transform|MakeTransform _returnvalue_2))
  (bind _returnvalue_4 (Class|KismetMathLibrary|ConvertTransformtoRelative _returnvalue_3 _returnvalue))
  (bind (_location _rotation _scale) (Math|Transform|BreakTransform _returnvalue_4))
  (bind _asbp_znake_game_mode (Utilities|Casting|CastToBP_ZnakeGameMode (Game|GetGameMode)))
  (bind _output_get (Variables|Default|SetGameModeReference _asbp_znake_game_mode))
  (Variables|/Script/ZnakeProject.ZnakeGameMode|SetStartingSpeed _output_get (Variables|Default|GetSpeed))
  (if (== Index 0)
    (bind _returnvalue_5 (Game|SpawnActorfromClass "/Game/Dynamic/Character/Behaviour/BP_SnakeBody.BP_SnakeBody_C" _returnvalue_4 "Undefined" 0 0))
    (Variables|/Script/ZnakeProject.SnakeBody|SetLastTransform _returnvalue_5 (Math|Transform|MakeTransform (+ _location "-32.000000, 0, 0") _rotation _scale))
    (Utilities|Array|Add (Variables|Default|GetBodyReferences) _returnvalue_5)
    (Variables|Default|SetNextBodyRef _returnvalue_5)
    (else
      (Class|SnakeCharacter|AddBodyPart))))

(fn SnakeGameOver
  (bind _asbp_znake_game_mode (Utilities|Casting|CastToBP_ZnakeGameMode (Game|GetGameMode)))
  (Default|GameOver _asbp_znake_game_mode))

(fn Accelerate
  (params (DeltaAcceleration :type Float%20%28single-precision%29))
  (bind _output_get (Variables|Default|SetAcceleration (+ (Variables|Default|GetAcceleration) DeltaAcceleration)))
  (return _output_get))

(fn DeltaSpeedtoAcceleration
  (params (DeltaSpeed :type Float%20%28single-precision%29) (TransionDuration :type Float%20%28single-precision%29))
  (bind _gamemodereference (Variables|Default|GetGameModeReference))
  (return (/ (Math|Float|Clamp(Float) DeltaSpeed (- (Variables|/Script/ZnakeProject.ZnakeGameMode|GetMinSpeed _gamemodereference) (Variables|Default|GetSpeed)) (- (Variables|/Script/ZnakeProject.ZnakeGameMode|GetMaxSpeed _gamemodereference) (Variables|Default|GetSpeed))) TransionDuration)))