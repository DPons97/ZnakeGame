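; BP_SnakeBody is one body segment of a tile-based snake, chained to the segment behind it by an object reference.
; MoveToNextTile saves the current transform, teleports to the given one, then recursively passes the saved transform down the chain like a linked list.
; AppendBody spawns a new segment, moves it to this segment's previous transform, links it as the next body and returns it.
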(fn ConstructionScript)

(fn MovetoNextTile
  (params (NextTransform :type Transform))
  (bind _nextbodyreference (Variables|Default|GetNextBodyReference))
  (Variables|Default|SetLastTransform (Transformation|GetActorTransform))
  (Transformation|SetActorTransform NextTransform false true)
  (Utilities|IsValid _nextbodyreference
    (:Is%20Valid
      (CallFunction|MovetoNextTile _nextbodyreference (Variables|Default|GetLastTransform)))))

(fn AppendBody
  (bind _returnvalue (Game|SpawnActorfromClass "BP_SnakeBody_C" (Class|KismetMathLibrary|ConvertTransformtoRelative (Math|Transform|MakeTransform (Math|Vector|MakeVector 32.0 0.0 0.0)) (Transformation|GetActorTransform)) "AlwaysSpawn" 0 0))
  (CallFunction|MovetoNextTile _returnvalue (Variables|Default|GetLastTransform))
  (bind _output_get (Variables|Default|SetNextBodyReference _returnvalue))
  (return _output_get))