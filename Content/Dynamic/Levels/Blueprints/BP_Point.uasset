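; BP_Point is a collectible point in the Znake snake game that grows the snake and raises the score.
; When a Player-tagged actor overlaps its ScoreBox, it adds a body part to the snake character, increments the game mode's Score and destroys itself.
; It disables spawning on the current map at BeginPlay and re-enables it on pickup, with a ToBeDeleted flag guarding against repeat pickups.
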(event OnComponentBeginOverlap(ScoreBox)
  (params (OverlappedComponent :type Primitive%20Component%20Object%20Reference) (OtherActor :type Actor%20Object%20Reference) (OtherComp :type Primitive%20Component%20Object%20Reference) (OtherBodyIndex :type Integer) (bFromSweep :type Boolean) (SweepResult :type Hit%20Result%20Structure%20%28by%20ref%29))
  (if (and (Actor|ActorHasTag OtherActor "Player") (not (Variables|Default|GetToBeDeleted)))
    (bind _asbp_snake_character (Utilities|Casting|CastToBP_SnakeCharacter OtherActor))
    (Default|AddBodyPart _asbp_snake_character)
    (CallFunction|IncreaseScoreandDestroy)))

(event EventBeginPlay
  (bind _asbp_znake_game_mode (Utilities|Casting|CastToBP_ZnakeGameMode (Game|GetGameMode)))
  (Variables|/Script/ZnakeProject.DefaultMap|SetEnableSpawning (Variables|/Game/Dynamic/Core/BP_ZnakeGameMode.BP_ZnakeGameMode_C|GetCurrentMap _asbp_znake_game_mode) false))

(fn ConstructionScript)

(fn IncreaseScoreandDestroy
  (bind _asbp_znake_game_mode (Utilities|Casting|CastToBP_ZnakeGameMode (Game|GetGameMode)))
  (bind _result (Math|Integer|IncrementInt (Variables|/Game/Dynamic/Core/BP_ZnakeGameMode.BP_ZnakeGameMode_C|GetScore _asbp_znake_game_mode))
    (:%20%20
      (Variables|/Game/Dynamic/Core/BP_ZnakeGameMode.BP_ZnakeGameMode_C|SetScore _asbp_znake_game_mode _result)
      (Variables|Default|SetToBeDeleted true)
      (Variables|/Script/ZnakeProject.DefaultMap|SetEnableSpawning (Variables|/Game/Dynamic/Core/BP_ZnakeGameMode.BP_ZnakeGameMode_C|GetCurrentMap _asbp_znake_game_mode) true)
      (Actor|DestroyActor))))