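; BP_Grass_1 is a tile map Blueprint with four teleporter triggers that move the player.
; Each trigger's begin-overlap event checks the other actor for the Player tag, then calls TeleportTo with that trigger and its matching TeleportTarget.
; The teleport logic itself is not defined in these graphs, and the construction script is empty.
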(event OnComponentBeginOverlap(Teleporter2)
  (params (OverlappedComponent :type Primitive%20Component%20Object%20Reference) (OtherActor :type Actor%20Object%20Reference) (OtherComp :type Primitive%20Component%20Object%20Reference) (OtherBodyIndex :type Integer) (bFromSweep :type Boolean) (SweepResult :type Hit%20Result%20Structure%20%28by%20ref%29))
  (if (Actor|ActorHasTag OtherActor "Player")
    (Class|Layer1Actor|Teleportto OverlappedComponent (Variables|Default|GetTeleportTarget2))))

(event OnComponentBeginOverlap(Teleporter3)
  (params (OverlappedComponent :type Primitive%20Component%20Object%20Reference) (OtherActor :type Actor%20Object%20Reference) (OtherComp :type Primitive%20Component%20Object%20Reference) (OtherBodyIndex :type Integer) (bFromSweep :type Boolean) (SweepResult :type Hit%20Result%20Structure%20%28by%20ref%29))
  (if (Actor|ActorHasTag OtherActor "Player")
    (Class|Layer1Actor|Teleportto OverlappedComponent (Variables|Default|GetTeleportTarget3))))

(event OnComponentBeginOverlap(Teleporter4)
  (params (OverlappedComponent :type Primitive%20Component%20Object%20Reference) (OtherActor :type Actor%20Object%20Reference) (OtherComp :type Primitive%20Component%20Object%20Reference) (OtherBodyIndex :type Integer) (bFromSweep :type Boolean) (SweepResult :type Hit%20Result%20Structure%20%28by%20ref%29))
  (if (Actor|ActorHasTag OtherActor "Player")
    (Class|Layer1Actor|Teleportto OverlappedComponent (Variables|Default|GetTeleportTarget4))))

(event OnComponentBeginOverlap(Teleporter1)
  (params (OverlappedComponent :type Primitive%20Component%20Object%20Reference) (OtherActor :type Actor%20Object%20Reference) (OtherComp :type Primitive%20Component%20Object%20Reference) (OtherBodyIndex :type Integer) (bFromSweep :type Boolean) (SweepResult :type Hit%20Result%20Structure%20%28by%20ref%29))
  (if (Actor|ActorHasTag OtherActor "Player")
    (Class|Layer1Actor|Teleportto OverlappedComponent (Variables|Default|GetTeleportTarget1))))

(fn ConstructionScript)