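; BP_SpeedBoost is a malus actor that applies a temporary speed boost to the snake character when its score-taken event fires.
; On BeginPlay it caches the player pawn and has it convert boost intensity and transition duration into an acceleration.
; A chain of delays applies and cancels that acceleration to ramp speed up, hold it for the boost duration, then ramp it back down symmetrically.
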(event Custom|ScoreTaken
  (bind _characterreference (Variables|Default|GetCharacterReference))
  (Utilities|FlowControl|Delay 0.01)
  (Default|Accelerate _characterreference (Variables|Default|GetBoostAcceleration))
  (Utilities|FlowControl|Delay (Variables|Default|GetTransitionDuration))
  (Default|Accelerate _characterreference (- 0.0 (Variables|Default|GetBoostAcceleration)))
  (Utilities|FlowControl|Delay (Variables|Default|GetBoostDuration))
  (Default|Accelerate _characterreference (- 0.0 (Variables|Default|GetBoostAcceleration)))
  (Utilities|FlowControl|Delay (Variables|Default|GetTransitionDuration))
  (Default|Accelerate _characterreference (Variables|Default|GetBoostAcceleration)))

(event EventBeginPlay
  (EventDispatchers|BindEventtoOnScoreTaken (delegate Custom|ScoreTaken))
  (bind _asbp_snake_character (Utilities|Casting|CastToBP_SnakeCharacter (Game|Player|GetPlayerPawn 0)))
  (bind _output_get (Variables|Default|SetCharacterReference _asbp_snake_character))
  (bind _acceleration (Default|DeltaSpeedtoAcceleration _output_get (Variables|Default|GetBoostIntensity) (Variables|Default|GetTransitionDuration)))
  (Variables|Default|SetBoostAcceleration _acceleration))

(fn ConstructionScript)