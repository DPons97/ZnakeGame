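; BP_PointRain is a bonus in the Znake game that rains extra points onto the map once its score is taken.
; The OnScoreTaken handler gets the current map from BP_ZnakeGameMode and looks up the "DefaultPoint" spawn index by name.
; A delayed loop then spawns those points one by one at random map locations until PointsToSpawn reaches zero or no location is found.
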(event Custom|ScoreTaken
  (bind _asbp_znake_game_mode (Utilities|Casting|CastToBP_ZnakeGameMode (Game|GetGameMode)))
  (bind (_outindex _returnvalue) (Class|DefaultMap|GetParamIndexbyName (Variables|/Script/ZnakeProject.ZnakeGameMode|GetCurrentMap _asbp_znake_game_mode) "DefaultPoint"))
  (if _returnvalue
    (if (!= (Variables|Default|GetPointsToSpawn) 0) :!label _label
      (bind (_outlocation _returnvalue_2) (Class|DefaultMap|ChooseRandomLocation (Variables|/Script/ZnakeProject.ZnakeGameMode|GetCurrentMap _asbp_znake_game_mode)))
      (if _returnvalue_2
        (Class|DefaultMap|SpawnPointActorbyIndex (Variables|/Script/ZnakeProject.ZnakeGameMode|GetCurrentMap _asbp_znake_game_mode) _outindex _outlocation)
        (Math|Integer|DecrementInt (Variables|Default|GetPointsToSpawn)
          (:%20%20
            (Utilities|FlowControl|Delay 0.2)
            (goto _label)))))))

(event EventBeginPlay
  (EventDispatchers|BindEventtoOnScoreTaken (delegate Custom|ScoreTaken)))

(fn ConstructionScript)