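; Ability Blueprint that temporarily changes the snake character's speed, named as a deceleration, when activated.
; On BeginPlay it caches the player's BP_SnakeCharacter and has it convert DeltaSpeed and TransitionDuration into an acceleration.
; On activation, timed opposing Accelerate calls ramp the speed, hold it for Duration, then ramp it back.
; Each ramp ends by applying the opposite value, so the net acceleration returns to zero.
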(event Custom|AbilityUsed
  (bind _characterreference (Variables|Default|GetCharacterReference))
  (Utilities|FlowControl|Delay 0.01)
  (Default|Accelerate _characterreference (Variables|Default|GetDeceleration))
  (Utilities|FlowControl|Delay (Variables|Default|GetTransitionDuration))
  (Default|Accelerate _characterreference (- 0.0 (Variables|Default|GetDeceleration)))
  (Utilities|FlowControl|Delay (Variables|Default|GetDuration))
  (Default|Accelerate _characterreference (- 0.0 (Variables|Default|GetDeceleration)))
  (Utilities|FlowControl|Delay (Variables|Default|GetTransitionDuration))
  (Default|Accelerate _characterreference (Variables|Default|GetDeceleration)))

(event EventBeginPlay
  (EventDispatchers|AssignOnAbilityActivated (delegate Custom|AbilityUsed))
  (bind _asbp_snake_character (Utilities|Casting|CastToBP_SnakeCharacter (Game|Player|GetPlayerPawn 0)))
  (bind _output_get (Variables|Default|SetCharacterReference _asbp_snake_character))
  (bind _acceleration (Default|DeltaSpeedtoAcceleration _output_get (Variables|Default|GetDeltaSpeed) (Variables|Default|GetTransitionDuration)))
  (Variables|Default|SetDeceleration _acceleration))

(fn ConstructionScript)